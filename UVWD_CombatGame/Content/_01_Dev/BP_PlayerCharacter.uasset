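; Player character Blueprint that routes incoming hits to its health component and carries a debug damage hotkey.
; The OnHit function passes its damage value straight to BPHealthComponent.
; Pressing 1 finds every BP_Character_Base actor, applies fixed damage through each one's health component, then prints a test message.
; BeginPlay, overlap and Tick are disabled stubs, and construction only calls the parent.
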(event EventBeginPlay
  (|CallParentFunction) ; This node is disabled and will not be called.\nDrag off pins to build functionality.
)

(event Collision|EventActorBeginOverlap
  (params (OtherActor :type Actor%20Object%20Reference)))

(event EventTick
  (params (DeltaSeconds :type Float%20%28single-precision%29)))

(event Input|KeyboardEvents|1
  (params (Key :type Key%20Structure :default "None"))
  (:Pressed
    (bind _outactors (Actor|GetAllActorsOfClass "/Game/_01_Dev/BP_Character_Base.BP_Character_Base_C"))
    (for _array_element _outactors
      (Default|Damage (Variables|/Game/_01_Dev/BP_Character_Base.BP_Character_Base_C|GetBP_HealthComponent _array_element) 2e+01))
    (Development|PrintString "HOI" true true "(R=1.000000,G=0.253117,B=0.352914,A=1.000000)")))

(fn ConstructionScript
  (|CallParentFunction))

(fn OnHit
  (params (Damage :type Float%20%28double-precision%29))
  (Default|Damage (Variables|Default|GetBP_HealthComponent) Damage))