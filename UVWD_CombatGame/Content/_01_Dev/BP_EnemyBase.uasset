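; Base enemy Blueprint that gives the enemy's AI a reference to another boss.
; On BeginPlay it runs the parent logic, then calls SetBossRefInBlackboard.
; That function gets the Blackboard through the enemy's AI Controller and writes OtherBoss as an object value under OtherBossKeyName.
; It has no active tick or overlap logic, and construction only calls the parent.
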(event EventBeginPlay
  (|CallParentFunction)
  (CallFunction|SetBossRefinBlackboard))

(event Collision|EventActorBeginOverlap
  (params (OtherActor :type Actor%20Object%20Reference)))

(event EventTick
  (params (DeltaSeconds :type Float%20%28single-precision%29)))

(fn ConstructionScript
  (|CallParentFunction))

(fn SetBossRefinBlackboard
  (AI|Components|Blackboard|SetValueasObject (AI|GetBlackboard (AI|GetAIController self)) (Variables|Default|GetOtherBossKeyName) (Variables|Default|GetOtherBoss)))