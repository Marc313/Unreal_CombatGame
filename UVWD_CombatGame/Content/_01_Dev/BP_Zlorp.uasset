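; Zlorp character Blueprint that specializes a parent class with its own HUD health bar and area-attack effect.
; Its Healthbar event finds the UIManager actor and assigns the HUD widget's Zlorp bar to BPHealthComponent.
; The PlayAreaAttackVFX override runs the parent version, then spawns an enlarged Priest wave particle at GroundFXPos.
; BeginPlay and Tick are empty, and the player-distance print and UI creation binding are unconnected.
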(event Custom|Healthbar
  (bind _returnvalue (Actor|GetActorOfClass "/Game/_01_Dev/UIManager.UIManager_C"))
  (Variables|/Game/_01_Dev/Health/BP_HealthComponent.BP_HealthComponent_C|SetHealthbar (Variables|Default|GetBP_HealthComponent) (Variables|/Game/_03_UI/Healthbar.Healthbar_C|GetZlorp (Variables|/Game/_01_Dev/UIManager.UIManager_C|GetHUD%20Widget _returnvalue))))

(event EventBeginPlay)

(event EventTick
  (params (DeltaSeconds :type Float%20%28single-precision%29)))

(fn ConstructionScript
  (|CallParentFunction))

(fn PlayAreaAttackVFX
  (bind _groundfx_pos (Variables|Default|GetGroundFX_Pos))
  (bind _returnvalue (Transformation|GetWorldTransform _groundfx_pos))
  (|CallParentFunction)
  (Effects|SpawnEmitteratLocation "/Game/RPGEffects/Particles/P_Priest_Wave.P_Priest_Wave" (.location _returnvalue) (.rotation _returnvalue) "2.000000,2.000000,2.000000"))