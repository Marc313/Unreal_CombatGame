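; Health component that tracks an actor's health, mirrors it on a health bar and signals death.
; Health starts at MaxHealth on BeginPlay, and each Damage call subtracts from it without clamping.
; Both steps push the health ratio to the Healthbar reference, which is not assigned here.
; OnDeath fires on any Damage call that leaves health at or below zero, so it can repeat.
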(event EventBeginPlay
  (Variables|Default|SetHealth (Variables|Default|GetMaxHealth))
  (bind _ratio (CallFunction|GetHealthRatio))
  (Progress|SetPercent (Variables|Default|GetHealthbar) _ratio))

(fn Damage
  (params (Damage :type Float%20%28double-precision%29))
  (bind _output_get (Variables|Default|SetHealth (- (Variables|Default|GetHealth) Damage)))
  (bind _ratio (CallFunction|GetHealthRatio))
  (Progress|SetPercent (Variables|Default|GetHealthbar) _ratio)
  (if (<= _output_get 0.0)
    (Default|CallOnDeath)))

(fn GetHealthRatio
  (return (/ (Variables|Default|GetHealth) (Variables|Default|GetMaxHealth))))