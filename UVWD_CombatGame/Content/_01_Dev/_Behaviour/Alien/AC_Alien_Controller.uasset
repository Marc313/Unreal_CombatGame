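; AI controller for the Alien boss that starts BT_Alien_Tree on BeginPlay and feeds movement angle to its animation.
; Each Tick finds a BP_Alien via GetActorOfClass, not the controlled pawn, and writes the angle between its forward vector and blackboard MoveDirection to MoveAngle.
; That angle, unsigned because it comes from acos of a dot product, then drives ABP_Alien through SetBSAngle.
; Debug prints of both bosses' states are disabled.
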(event EventBeginPlay
  (AI|RunBehaviorTree "/Game/_01_Dev/_Behaviour/Alien/BT_Alien_Tree.BT_Alien_Tree"))

(event EventTick
  (params (DeltaSeconds :type Float%20%28single-precision%29))
  (bind _returnvalue (AI|GetBlackboard 0))
  (bind _returnvalue_2 (AI|GetBlackboard 0))
  (Utilities|FlowControl|Sequence
    (:then_0
      (bind _returnvalue_3 (Actor|GetActorOfClass "/Game/_01_Dev/BP_Alien.BP_Alien_C"))
      (bind _asbp_character_base (Utilities|Casting|CastToBP_Character_Base _returnvalue_3))
      (Utilities|FlowControl|Sequence
        (:then_0
          (AI|Components|Blackboard|SetValueasFloat _returnvalue_2 (Utilities|Name|MakeLiteralName "MoveAngle") (Class|KismetMathLibrary|DegAcos (Math|Vector|DotProduct (Math|Vector|Normalize (Math|Vector|GetForwardVector (Variables|/Script/Engine.Character|GetCapsuleComponent _asbp_character_base))) (Math|Vector|Normalize (AI|Components|Blackboard|GetValueasVector _returnvalue_2 (Utilities|Name|MakeLiteralName "MoveDirection")))))))
        (:then_1
          (bind _asabp_alien (Utilities|Casting|CastToABP_Alien (Components|SkeletalMesh|GetAnimInstance (Variables|/Script/Engine.Character|GetMesh _asbp_character_base))))
          (Default|SetBSAngle _asabp_alien (Class|BlackboardComponent|GetValueasFloat _returnvalue_2 (Utilities|Name|MakeLiteralName "MoveAngle"))))))
    (:then_1
      (Development|PrintString (Utilities|String|ToString(Byte) (Class|BlackboardComponent|GetValueasEnum _returnvalue (Utilities|Name|MakeLiteralName "OtherBossState"))) true true "(R=0.997650,G=1.000000,B=0.000000,A=1.000000)")
      (bind _asbp_character_base_2 (Utilities|Casting|CastToBP_Character_Base (AI|Components|Blackboard|GetValueasObject _returnvalue (Utilities|Name|MakeLiteralName "OtherBoss"))))
      (Development|PrintString (Utilities|String|ToString(Byte) (Class|BlackboardComponent|GetValueasEnum (AI|GetBlackboard (AI|GetAIController _asbp_character_base_2)) (Utilities|Name|MakeLiteralName "BossState"))) true true "(R=1.000000,G=0.058924,B=0.849261,A=1.000000)"))))

(fn ConstructionScript)