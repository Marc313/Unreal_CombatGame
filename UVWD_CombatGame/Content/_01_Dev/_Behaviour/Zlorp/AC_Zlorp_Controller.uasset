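; AI controller for the Zlorp enemy that runs its behavior tree and feeds movement direction into its animation.
; Each Tick it looks up the BP_Zlorp actor by class, rather than using the controlled pawn.
; It computes the unsigned angle between the capsule's forward vector and the blackboard MoveDirection and stores it as MoveAngle.
; That angle is then passed to the ABP_EnemyBase anim instance as the blendspace angle.
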(event EventBeginPlay
  (AI|RunBehaviorTree "/Game/_01_Dev/_Behaviour/Zlorp/BT_Zlorp_Tree.BT_Zlorp_Tree"))

(event EventTick
  (params (DeltaSeconds :type Float%20%28single-precision%29))
  (bind _returnvalue (AI|GetBlackboard 0))
  (Utilities|FlowControl|Sequence
    (:then_0
      (bind _returnvalue_2 (Actor|GetActorOfClass "/Game/_01_Dev/BP_Zlorp.BP_Zlorp_C"))
      (bind _asbp_character_base (Utilities|Casting|CastToBP_Character_Base _returnvalue_2))
      (Utilities|FlowControl|Sequence
        (:then_0
          (AI|Components|Blackboard|SetValueasFloat _returnvalue (Utilities|Name|MakeLiteralName "MoveAngle") (Class|KismetMathLibrary|DegAcos (Math|Vector|DotProduct (Math|Vector|Normalize (Math|Vector|GetForwardVector (Variables|/Script/Engine.Character|GetCapsuleComponent _asbp_character_base))) (Math|Vector|Normalize (AI|Components|Blackboard|GetValueasVector _returnvalue (Utilities|Name|MakeLiteralName "MoveDirection")))))))
        (:then_1
          (bind _asabp_enemy_base (Utilities|Casting|CastToABP_EnemyBase (Components|SkeletalMesh|GetAnimInstance (Variables|/Script/Engine.Character|GetMesh _asbp_character_base)))
            (:then
              (Default|SetBSAngle _asabp_enemy_base (Class|BlackboardComponent|GetValueasFloat _returnvalue (Utilities|Name|MakeLiteralName "MoveAngle"))))
            (:CastFailed
              (Development|PrintString "failed"))))))))

(fn ConstructionScript)