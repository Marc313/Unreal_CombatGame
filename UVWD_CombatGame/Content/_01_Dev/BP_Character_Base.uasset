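; Base character Blueprint providing health, death and attack helpers, with death only printing a debug message.
; BeginPlay binds the health component's death event, and OnHit forwards damage to that component.
; Area (sphere overlap) and beam (debug-drawn single sphere trace) attacks feed HitTargets, which damages player characters but calls its own OnHit for other BP_Character_Base targets.
; GetRandomAttack picks a montage; PlayAreaAttackVFX is an empty stub.
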(event Custom|Death
  (CallFunction|OnDeath))

(event EventBeginPlay
  (EventDispatchers|BindEventtoOnDeath (Variables|Default|GetBP_HealthComponent) (delegate Custom|Death)))

(fn ConstructionScript)

(fn AreaOfAttack
  (params (AreaRadius :type Float%20%28double-precision%29) (Damage :type Float%20%28double-precision%29) (LocationOffset :type Vector))
  (bind _outactors (Collision|SphereOverlapActors (+ LocationOffset (Transformation|GetWorldLocation (Variables|Character|GetMesh))) AreaRadius (Utilities|Array|MakeArray "ObjectTypeQuery3") 0))
  (CallFunction|HitTargets Damage _outactors))

(fn PlayAreaAttackVFX)

(fn OnHit
  (params (Damage :type Float%20%28double-precision%29))
  (Default|Damage (Variables|Default|GetBP_HealthComponent) Damage))

(fn GetRandomAttack
  (return (.OutItem (Utilities|Array|Random (Variables|Default|GetAttackMontages)))))

(fn OnDeath
  (Development|PrintString "DEAD"))

(fn HitTargets
  (params (Damage :type Float%20%28double-precision%29) (Targets :type Array%20of%20Actor%20Object%20References))
  (for _array_element Targets
    (bind _asbp_player_character (Utilities|Casting|CastToBP_PlayerCharacter _array_element)
      (:then
        (Default|OnHit _asbp_player_character Damage))
      (:CastFailed
        (Utilities|Casting|CastToBP_Character_Base _array_element)
        (CallFunction|OnHit Damage)))))

(fn BeamAttack
  (params (BeamRadius :type Float%20%28double-precision%29) (LocationOffset :type Vector) (Damage :type Float%20%28double-precision%29) (EndLocationOffset :type Float%20%28double-precision%29))
  (bind _returnvalue (Transformation|GetActorLocation))
  (bind _outhit (Collision|SphereTraceForObjects (+ (* LocationOffset "") _returnvalue) (+ (* EndLocationOffset (Math|Vector|GetRightVector (Variables|Character|GetMesh))) _returnvalue) BeamRadius (Utilities|Array|MakeArray "ObjectTypeQuery3") false 0 "ForDuration"))
  (CallFunction|HitTargets Damage (Utilities|Array|MakeArray (.hitactor _outhit))))