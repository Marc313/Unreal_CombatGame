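; BP_Door is an interactive door that the player swings open and closed with the E key.
; An OpenTrigger overlap with the third-person character enables input on the door for player 0, and leaving the trigger disables it.
; Each E press alternates through a FlipFlop between playing and reversing DoorTimeline, whose DoorOpen track drives the door's relative yaw.
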(event OnComponentBeginOverlap(OpenTrigger)
  (params (OverlappedComponent :type Primitive%20Component%20Object%20Reference) (OtherActor :type Actor%20Object%20Reference) (OtherComp :type Primitive%20Component%20Object%20Reference) (OtherBodyIndex :type Integer) (bFromSweep :type Boolean) (SweepResult :type Hit%20Result%20Structure%20%28by%20ref%29))
  ;[1 1 1] Collision
  (Utilities|Casting|CastToBP_ThirdPersonCharacter OtherActor)
  (Input|EnableInput (Game|GetPlayerController 0)))

(event OnComponentEndOverlap(OpenTrigger)
  (params (OverlappedComponent :type Primitive%20Component%20Object%20Reference) (OtherActor :type Actor%20Object%20Reference) (OtherComp :type Primitive%20Component%20Object%20Reference) (OtherBodyIndex :type Integer))
  ;[1 1 1] Collision
  (Utilities|Casting|CastToBP_ThirdPersonCharacter OtherActor)
  (Input|DisableInput (Game|GetPlayerController 0) 0))

(event Input|KeyboardEvents|E
  (params (Key :type Key%20Structure :default "None"))
  ;[1 1 1] OnInteract
  (:Pressed
    (Utilities|FlowControl|FlipFlop
      (:A
        (bind _door_open (Timeline|Door%20Timeline Play)
          (:Update
            (Transformation|SetRelativeRotation (Variables|Default|GetDoor) (Math|Rotator|MakeRotator 0.0 0.0 _door_open) false false))))
      (:B
        (Timeline|Door%20Timeline Reverse)))))

(fn ConstructionScript)