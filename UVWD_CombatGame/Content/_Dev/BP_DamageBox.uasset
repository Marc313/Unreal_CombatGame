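; BP_DamageBox is a fire hazard volume that damages a BP_ThirdPersonCharacter inside its Box collision.
; BeginPlay spawns a persistent, scaled-up fire emitter at the actor's location.
; Entering applies EnterDamage, stores that character and starts a looping one-second timer that applies Damage to it.
; Any end overlap clears the timer, without checking which actor left.
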(event OnComponentBeginOverlap(Box)
  (params (OverlappedComponent :type Primitive%20Component%20Object%20Reference) (OtherActor :type Actor%20Object%20Reference) (OtherComp :type Primitive%20Component%20Object%20Reference) (OtherBodyIndex :type Integer) (bFromSweep :type Boolean) (SweepResult :type Hit%20Result%20Structure%20%28by%20ref%29))
  ;[1 1 1] Initial Enter Damage
  (bind _asbp_third_person_character (Utilities|Casting|CastToBP_ThirdPersonCharacter OtherActor))
  (Game|Damage|ApplyDamage _asbp_third_person_character (Variables|Default|GetEnterDamage) 0 0)
  ;[1 1 1] Initialize Damage over time
  (Variables|Default|SetAs%20BP%20Third%20Person%20Character _asbp_third_person_character)
  (bind _returnvalue (Utilities|Time|SetTimerbyEvent (delegate Custom|DamagePlayer) 1.0 true))
  (Variables|Default|SetDamageTimer _returnvalue))

(event OnComponentEndOverlap(Box)
  (params (OverlappedComponent :type Primitive%20Component%20Object%20Reference) (OtherActor :type Actor%20Object%20Reference) (OtherComp :type Primitive%20Component%20Object%20Reference) (OtherBodyIndex :type Integer))
  ;[1 1 1] Disable Damage Timer
  (Utilities|Time|ClearandInvalidateTimerbyHandle (Variables|Default|GetDamageTimer)))

(event Custom|DamagePlayer
  ;[1 1 1] Initialize Damage over time
  (Game|Damage|ApplyDamage (Variables|Default|GetAs%20BP%20Third%20Person%20Character) (Variables|Default|GetDamage) 0 0))

(event EventBeginPlay
  (Effects|SpawnEmitteratLocation "/Game/StarterContent/Particles/P_Fire.P_Fire" (Transformation|GetActorLocation) "0, 0, 0" "3.000000,3.000000,3.000000" false))

(fn ConstructionScript)